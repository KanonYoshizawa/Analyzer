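; Battle1 is a battle setup actor that spawns a group of enemies at play start and offers key controls to inspect and alter their stats.
; BeginPlay fills a class array with three NewBlueprint1 entries, then 新規関数 spawns them in a row along Y and stores the instances in Battle1Enemy.
; E prints each enemy's Status struct values, while R rebuilds the first enemy's struct with increased HP.
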(event EventBeginPlay
  (Variables|Default|SetBattle1 (Utilities|Array|MakeArray "/Game/Analyzer/Blueprint/NewBlueprint1.NewBlueprint1_C" "/Game/Analyzer/Blueprint/NewBlueprint1.NewBlueprint1_C" "/Game/Analyzer/Blueprint/NewBlueprint1.NewBlueprint1_C"))
  (CallFunction|新規関数)
  (Input|EnableInput (Game|GetPlayerController 0)))

(event Input|KeyboardEvents|E
  (params (Key :type Key%20Structure :default "None"))
  (:Pressed
    (for _array_element (Variables|Default|GetBattle1Enemy)
      (Development|PrintString (Utilities|String|Append (Utilities|String|ToString(Integer) (.enemyhp (Variables|/Game/Analyzer/Blueprint/Enemy.Enemy_C|GetStatus _array_element))) (Utilities|String|ToString(Integer) (.enemyatk (Variables|/Game/Analyzer/Blueprint/Enemy.Enemy_C|GetStatus _array_element))) (Utilities|String|ToString(Integer) (.enemydef (Variables|/Game/Analyzer/Blueprint/Enemy.Enemy_C|GetStatus _array_element))) (Utilities|String|ToString(Integer) (.enemyspd (Variables|/Game/Analyzer/Blueprint/Enemy.Enemy_C|GetStatus _array_element))))))))

(event Input|KeyboardEvents|R
  (params (Key :type Key%20Structure :default "None"))
  (bind _battle1enemy (Variables|Default|GetBattle1Enemy))
  (bind _output (Utilities|Array|Get(acopy) _battle1enemy))
  (:Pressed
    (Variables|/Game/Analyzer/Blueprint/Enemy.Enemy_C|SetStatus _output (Utilities|Struct|MakeNewUserDefinedStruct (+ (.enemyhp (Variables|/Game/Analyzer/Blueprint/Enemy.Enemy_C|GetStatus _output)) 10) (.enemyatk (Variables|/Game/Analyzer/Blueprint/Enemy.Enemy_C|GetStatus _output)) (.enemydef (Variables|/Game/Analyzer/Blueprint/Enemy.Enemy_C|GetStatus _output)) (.enemyspd (Variables|/Game/Analyzer/Blueprint/Enemy.Enemy_C|GetStatus _output))))))

(fn ConstructionScript)

(fn 新規関数
  (for (_array_element _array_index) (Variables|Default|GetBattle1)
    (bind _returnvalue (Game|SpawnActorfromClass _array_element (Math|Transform|MakeTransform (Math|Vector|MakeVector 4e+02 (+ (* _array_index 2.5e+02) (Math|Float|MakeLiteralFloat -2.5e+02)) 5e+01)) "Undefined" "MultiplyWithRoot" 0 0))
    (Utilities|Array|SetArrayElem (Variables|Default|GetBattle1Enemy) _array_index _returnvalue true)))